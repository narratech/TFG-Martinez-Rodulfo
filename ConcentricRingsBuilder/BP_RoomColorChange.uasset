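; Dungeon Architect selector rule for the concentric rings builder that selects theme nodes lying in one ring, likely for recoloring rooms.
; SelectNode measures each grid position's distance from a fixed offset center and accepts it within a band derived from CheckRing, RingRadius and RadiusFraction.
; Band edges come from diagonal and axis-aligned corner distances with slight padding; ring zero starts at the center.
; The EventGraph holds an unexecuted copy of this logic.
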(fn `SelectNode`
  (params (Model :type "GridDungeonModel Object Reference") (Config :type "GridDungeonConfig Object Reference") (Builder :type "GridDungeonBuilder Object Reference") (Query :type "GridDungeonQuery Object Reference") (Cell :type "GridDungeonCell Structure (by ref)") (RandomStream :type "RandomStream Structure (by ref)") (GridX :type Integer) (GridY :type Integer) (MarkerTransform :type "Transform Structure (by ref)"))
  (returns (ReturnValue :type Boolean))
  (locals (CenterDistance :type "Float (double-precision)") (LowerRadius :type "Float (double-precision)") (UpperRadius :type "Float (double-precision)") (RadiusOffset :type "Float (double-precision)") (BaseRadius :type "Float (double-precision)"))
  (bind _ringradius (`self.RingRadius`))
  (bind _returnvalue (- (* (`KismetMathLibrary.DegCos` 45.0) (`local.BaseRadius`)) (`local.RadiusOffset`)))
  ;[1 1 1] Selection Logic
  (set `local.BaseRadius` (* (`self.CheckRing`) _ringradius))
  (set `local.RadiusOffset` (/ _ringradius (`self.RadiusFraction`)))
  (set `local.CenterDistance` (`KismetMathLibrary.Sqrt` (+ (`KismetMathLibrary.Square` (`KismetMathLibrary.Conv_IntToDouble` (+ GridX 3))) (`KismetMathLibrary.Square` (`KismetMathLibrary.Conv_IntToDouble` (+ GridY -3))))))
  (if (== (`self.CheckRing`) 0)
    (set `local.LowerRadius` 0.0)
    (else
      (set `local.LowerRadius` (- (`KismetMathLibrary.Sqrt` (+ (`KismetMathLibrary.Square` _returnvalue) (`KismetMathLibrary.Square` _returnvalue))) 5.0))))
  (set `local.UpperRadius` (+ (`KismetMathLibrary.Sqrt` (+ (`KismetMathLibrary.Square` (+ (`local.BaseRadius`) (`local.RadiusOffset`))) (`KismetMathLibrary.Square` (`local.RadiusOffset`)))) 5.0))
  (return (and (>= (`local.CenterDistance`) (`local.LowerRadius`)) (<= (`local.CenterDistance`) (`local.UpperRadius`)))))